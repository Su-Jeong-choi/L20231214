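; Player-controlled P-38 plane pawn that constantly moves along its forward vector and fires rockets.
; Pitch and Roll axes apply frame-rate-scaled local rotation, while Fire spawns BP_Rocket at the pawn's transform.
; BeginPlay registers PPRight twice with BPRotateSceneComponent's component list, with no other propeller added.
; The RotaintionPropeller helper rolls a given component by Speed but is not called in these graphs.
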(event EventBeginPlay
  (Utilities|Array|Add (Variables|/Game/Bluprints/BP_RotateSceneComponent.BP_RotateSceneComponent_C|GetSceneComponets (Variables|Default|GetBP_RotateSceneComponent)) (Variables|Default|GetPP_Right))
  (Utilities|Array|Add (Variables|/Game/Bluprints/BP_RotateSceneComponent.BP_RotateSceneComponent_C|GetSceneComponets (Variables|Default|GetBP_RotateSceneComponent)) (Variables|Default|GetPP_Right)))

(event Collision|EventActorBeginOverlap
  (params (OtherActor :type Actor%20Object%20Reference)))

(event EventTick
  (params (DeltaSeconds :type Float%20%28single-precision%29))
  (Pawn|Input|AddMovementInput (Transformation|GetActorForwardVector) 1.0 false))

(event Input|ActionEvents|InputActionFire
  (params (Key :type Key%20Structure :default "None"))
  (:Pressed
    (Game|SpawnActorfromClass "/Game/Bluprints/BP_Rocket.BP_Rocket_C" (Transformation|GetActorTransform) "AlwaysSpawn" "MultiplyWithRoot" 0 0)))

(event Input|AxisEvents|InputAxisPitch
  (params (AxisValue :type Float%20%28single-precision%29))
  (Transformation|AddActorLocalRotation (Math|Rotator|MakeRotator 0.0 (* AxisValue (Utilities|Time|GetWorldDeltaSeconds) (Variables|Default|GetRotateSpeed)) 0.0) false false))

(event Input|AxisEvents|InputAxisRoll
  (params (AxisValue :type Float%20%28single-precision%29))
  (Transformation|AddActorLocalRotation (Math|Rotator|MakeRotator (* AxisValue (Utilities|Time|GetWorldDeltaSeconds) (Variables|Default|GetRotateSpeed)) 0.0 0.0) false false))

(fn ConstructionScript)

(fn RotaintionPropeller
  (params (self2 :type Scene%20Component%20Object%20Reference))
  (Transformation|AddLocalRotation self2 (Math|Rotator|MakeRotator (* (Utilities|Time|GetWorldDeltaSeconds) (Variables|Default|GetSpeed)) 0.0 0.0) false false))